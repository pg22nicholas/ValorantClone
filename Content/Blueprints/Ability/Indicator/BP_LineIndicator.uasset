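; BP_LineIndicator is an ability indicator Blueprint that displays an animated line.
; On BeginPlay it scales the root by Width and the X component of LineDirection, then creates a dynamic material instance for the Line component.
; After a short delay, a timeline drives the material's LineValue parameter, with play rate set to the inverse of Length so Length controls the animation's duration.
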(event EventBeginPlay
  (bind _width (Variables|Default|GetWidth))
  (Utilities|FlowControl|Sequence
    (:then_0
      (Transformation|SetWorldScale3D (Variables|Default|GetDefaultSceneRoot) (Math|Vector|MakeVector _width (.x (Variables|Default|GetLineDirection)) _width)))
    (:then_1
      (bind _returnvalue (Rendering|Material|CreateDynamicMaterialInstance (Variables|Default|GetLine) :!class /Script/Engine.DecalComponent))
      (Variables|Default|SetLineRef _returnvalue))
    (:then_2
      (Components|Timeline|SetPlayRate (Variables|Default|GetLineValueTimeline) (/ 1.0 (Variables|Default|GetLength))))
    (:then_3
      (Utilities|FlowControl|Delay 0.1)
      (bind _linevalue (Timeline|LineValueTimeline Play)
        (:Update
          (Rendering|Material|SetScalarParameterValue (Variables|Default|GetLineRef) "LineValue" (* _linevalue 5.0) :!class /Script/Engine.MaterialInstanceDynamic))))))

(fn ConstructionScript)