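; BP_CircleIndicator is a circular ability indicator that shows an outline and an area fill animated over a set Length.
; On BeginPlay it scales its root from Radius and creates dynamic material instances for the Circum and Area components, using the Circum1Area0 parameter to set each role.
; After a brief delay, a timeline rate-scaled by Length drives the Area material's AreaValue parameter to animate the fill.
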(event EventBeginPlay
  (bind _radius (Variables|Default|GetRadius))
  (bind _returnvalue (/ _radius 0.5))
  (Utilities|FlowControl|Sequence
    (:then_0
      (Transformation|SetWorldScale3D (Variables|Default|GetDefaultSceneRoot) (Math|Vector|MakeVector _returnvalue _returnvalue _returnvalue)))
    (:then_1
      (bind _returnvalue_2 (Rendering|Material|CreateDynamicMaterialInstance (Variables|Default|GetCircum) :!class /Script/Engine.DecalComponent))
      (bind _output_get (Variables|Default|SetCircumRef _returnvalue_2))
      (Rendering|Material|SetScalarParameterValue _output_get "Circum1Area0" 1.0 :!class /Script/Engine.MaterialInstanceDynamic))
    (:then_2
      (bind _returnvalue_3 (Rendering|Material|CreateDynamicMaterialInstance (Variables|Default|GetArea) :!class /Script/Engine.DecalComponent))
      (bind _output_get_2 (Variables|Default|SetAreaRef _returnvalue_3))
      (Rendering|Material|SetScalarParameterValue _output_get_2 "Circum1Area0" 0.0 :!class /Script/Engine.MaterialInstanceDynamic))
    (:then_3
      (Components|Timeline|SetPlayRate (Variables|Default|GetAreaValueTimeline) (/ 1.0 (Variables|Default|GetLength))))
    (:then_4
      (Utilities|FlowControl|Delay 0.1)
      (bind _areavaluealpha (Timeline|AreaValueTimeline Play)
        (:Update
          (Rendering|Material|SetScalarParameterValue (Variables|Default|GetAreaRef) "AreaValue" (* _areavaluealpha 0.5) :!class /Script/Engine.MaterialInstanceDynamic))))))

(fn ConstructionScript)